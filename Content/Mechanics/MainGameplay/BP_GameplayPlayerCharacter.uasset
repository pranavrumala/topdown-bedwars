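; Playable gameplay character with Enhanced Input movement, jump, a launch-based dash, and melee and ranged attacks.
; On BeginPlay it grants test Gameplay Abilities, builds the health bar widget and caches the controller and player start.
; Attack inputs activate ground or air abilities depending on whether it is falling.
; Damage is filtered by temporarily stored hitbox IDs and updates the health bar, with death triggering a delayed respawn at the player start.
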(event Custom|Hitbox%20ID%20Removal
  ;[0.15 0.15 0.15 0.5] Prevent Attacks dealing damage more than once
  (Utilities|FlowControl|Delay 1.0)
  (Utilities|Array|RemoveIndex (Variables|Default|GetCurrent%20Hitbox%20IDs)))

(event Custom|Respawn%20Player
  (bind _max_health (Variables|Default|GetMax%20Health))
  ;[0.15 0.15 0.15 0.5] Handle Death and Respawn
  (Utilities|FlowControl|Delay 1.0)
  (bind _output_get (Variables|Default|SetHealth _max_health))
  (Variables|/Game/Mechanics/MainGameplay/WBP_HealthBar.WBP_HealthBar_C|SetHealthPercentage (Variables|Default|GetHealthBar%20Widget) (/ _output_get _max_health))
  (Transformation|SetActorTransform (Transformation|GetActorTransform (Variables|Default|GetPlayer%20Start)))
  (Input|EnableInput (Variables|Default|GetPlayer%20Controller)))

(event Input|EnhancedActionEvents|EnhancedInputActionIA_Move
  (params (ActionValue :type Vector%202D%20Structure) (ElapsedSeconds :type Float%20%28double-precision%29) (TriggeredSeconds :type Float%20%28double-precision%29) (InputAction :type Input%20Action%20Object%20Reference :default "/Game/Mechanics/MainGameplay/Input/IA_Move.IA_Move"))
  ;[0.1274 0 0.15 0.5] Inputs
  (Pawn|Input|AddMovementInput (Class|KismetMathLibrary|VectorRight) (.x ActionValue) false)
  (Pawn|Input|AddMovementInput (Class|KismetMathLibrary|VectorForward) (.y ActionValue) false))

(event Input|EnhancedActionEvents|EnhancedInputActionIA_Jump
  (params (ActionValue :type Boolean) (ElapsedSeconds :type Float%20%28double-precision%29) (TriggeredSeconds :type Float%20%28double-precision%29) (InputAction :type Input%20Action%20Object%20Reference :default "/Game/Mechanics/MainGameplay/Input/IA_Jump.IA_Jump"))
  ;[0.1274 0 0.15 0.5] Inputs
  (Character|Jump)
  (Rendering|SetVisibility (Variables|Default|GetWidget) true false))

(event Input|EnhancedActionEvents|EnhancedInputActionIA_Dash
  (params (ActionValue :type Boolean) (ElapsedSeconds :type Float%20%28double-precision%29) (TriggeredSeconds :type Float%20%28double-precision%29) (InputAction :type Input%20Action%20Object%20Reference :default "/Game/Mechanics/MainGameplay/Input/IA_Dash.IA_Dash"))
  ;[0.1274 0 0.15 0.5] Inputs
  (:Started
    (Character|LaunchCharacter (* (Class|Pawn|GetLastMovementInputVector) (Variables|Default|GetDash%20Velocity)) true true)))

(event Input|EnhancedActionEvents|EnhancedInputActionIA_Melee
  (params (ActionValue :type Boolean) (ElapsedSeconds :type Float%20%28double-precision%29) (TriggeredSeconds :type Float%20%28double-precision%29) (InputAction :type Input%20Action%20Object%20Reference :default "/Game/Mechanics/MainGameplay/Input/IA_Melee.IA_Melee"))
  (bind _abilitysystem (Variables|Default|GetAbilitySystem))
  ;[0.1274 0 0.15 0.5] Inputs
  (:Started
    (if (AI|Components|NavMovement|IsFalling (Variables|Character|GetCharacterMovement))
      (Abilities|TryActivateAbilitybyClass _abilitysystem "/Game/Mechanics/MainGameplay/Abilities/GA_TestAirMelee.GA_TestAirMelee_C" true)
      (else
        (Abilities|TryActivateAbilitybyClass _abilitysystem "/Game/Mechanics/MainGameplay/Abilities/GA_TestGroundMelee.GA_TestGroundMelee_C" true)))))

(event Input|EnhancedActionEvents|EnhancedInputActionIA_Ranged
  (params (ActionValue :type Boolean) (ElapsedSeconds :type Float%20%28double-precision%29) (TriggeredSeconds :type Float%20%28double-precision%29) (InputAction :type Input%20Action%20Object%20Reference :default "/Game/Mechanics/MainGameplay/Input/IA_Ranged.IA_Ranged"))
  (bind _abilitysystem (Variables|Default|GetAbilitySystem))
  ;[0.1274 0 0.15 0.5] Inputs
  (:Started
    (if (AI|Components|NavMovement|IsFalling (Variables|Character|GetCharacterMovement))
      (Abilities|TryActivateAbilitybyClass _abilitysystem "/Game/Mechanics/MainGameplay/Abilities/GA_TestAirRanged.GA_TestAirRanged_C" true)
      (else
        (Abilities|TryActivateAbilitybyClass _abilitysystem "/Game/Mechanics/MainGameplay/Abilities/GA_TestGroundRanged.GA_TestGroundRanged_C" true)))))

(event EventBeginPlay
  (CallFunction|GiveTestAbilities)
  (CallFunction|SetupHealthBarWidget)
  (Utilities|FlowControl|DelayUntilNextTick)
  (CallFunction|GetNecessaryVariables))

(event Collision|EventActorBeginOverlap
  (params (OtherActor :type Actor%20Object%20Reference)))

(event EventTick
  (params (DeltaSeconds :type Float%20%28single-precision%29)))

(event EventRecievedDamage
  (params (Damage :type Float%20%28double-precision%29) (ID :type Float%20%28double-precision%29))
  (bind _current_hitbox_ids (Variables|Default|GetCurrent%20Hitbox%20IDs))
  ;[0.15 0.15 0.15 0.5] Prevent Attacks dealing damage more than once
  (if (not (Utilities|Array|ContainsItem _current_hitbox_ids ID))
    (Utilities|Array|Add _current_hitbox_ids ID)
    (CallFunction|HitboxIDRemoval)
    ;[0.15 0.15 0.15 0.5] Damage Calculations and show on Health Bar
    (bind _output_get (Variables|Default|SetHealth (- (Variables|Default|GetHealth) Damage)))
    (Variables|/Game/Mechanics/MainGameplay/WBP_HealthBar.WBP_HealthBar_C|SetHealthPercentage (Variables|Default|GetHealthBar%20Widget) (/ _output_get (Variables|Default|GetMax%20Health)))
    ;[0.15 0.15 0.15 0.5] Handle Death and Respawn
    (if (<= (Variables|Default|GetHealth) 0.0)
      (Input|DisableInput (Variables|Default|GetPlayer%20Controller))
      (CallFunction|RespawnPlayer))))

(fn ConstructionScript)

(fn GiveTestAbilities
  (GameplayAbilities|GiveAbility (Variables|Default|GetAbilitySystem) "/Game/Mechanics/MainGameplay/Abilities/GA_TestGroundMelee.GA_TestGroundMelee_C" 0 -1)
  (GameplayAbilities|GiveAbility (Variables|Default|GetAbilitySystem) "/Game/Mechanics/MainGameplay/Abilities/GA_TestGroundRanged.GA_TestGroundRanged_C" 0 -1)
  (GameplayAbilities|GiveAbility (Variables|Default|GetAbilitySystem) "/Game/Mechanics/MainGameplay/Abilities/GA_TestAirMelee.GA_TestAirMelee_C" 0 -1)
  (GameplayAbilities|GiveAbility (Variables|Default|GetAbilitySystem) "/Game/Mechanics/MainGameplay/Abilities/GA_TestAirRanged.GA_TestAirRanged_C" 0 -1))

(fn SetupHealthBarWidget
  (bind _widget (Variables|Default|GetWidget))
  (bind _returnvalue (UserInterface|CreateWidget "/Game/Mechanics/MainGameplay/WBP_HealthBar.WBP_HealthBar_C"))
  (UserInterface|SetWidget _widget _returnvalue)
  (bind _aswbp_health_bar (Utilities|Casting|CastToWBP_HealthBar (UserInterface|GetWidget _widget))
    (:then
      (Variables|Default|SetHealthBar%20Widget _aswbp_health_bar))
    (:CastFailed
      (Development|PrintString "Cannot Get HealthBar"))))

(fn GetNecessaryVariables
  (Variables|Default|SetGame%20Mode (Game|GetGameMode))
  (bind _asplayer_controller (Utilities|Casting|CastToPlayerController (Pawn|GetController)))
  (Variables|Default|SetPlayer%20Controller _asplayer_controller)
  (Variables|Default|SetPlayer%20Start (Class|GameModeBase|FindPlayerStart (Variables|Default|GetGame%20Mode) (Variables|Default|GetPlayer%20Controller))))