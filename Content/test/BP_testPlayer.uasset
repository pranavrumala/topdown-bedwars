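; BP_testPlayer is a test player character that moves, aims, jumps and shoots through Enhanced Input, and returns to a player start when shot.
; Movement follows world axes, while the look axes become a control yaw through Atan2, in twin-stick style.
; Shooting spawns a BP_testBullet at the Scene component and sets the player as owner.
; Capsule overlap with another owner's "Bullet"-tagged actor teleports the player to the GameMode's chosen start.
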(event OnComponentBeginOverlap(CapsuleComponent)
  (params (OverlappedComponent :type Primitive%20Component%20Object%20Reference) (OtherActor :type Actor%20Object%20Reference) (OtherComp :type Primitive%20Component%20Object%20Reference) (OtherBodyIndex :type Integer) (bFromSweep :type Boolean) (SweepResult :type Hit%20Result%20Structure%20%28by%20ref%29))
  (if (Actor|ActorHasTag OtherActor "Bullet")
    (if (!= (Components|GetOwner OtherActor) self)
      (Transformation|SetActorTransform self (Transformation|GetActorTransform (Class|GameModeBase|FindPlayerStart (Variables|Default|GetGame%20Mode) (Variables|Default|GetPlayer%20Controller)))))))

(event Input|EnhancedActionEvents|EnhancedInputActionIA_Movetest
  (params (ActionValue :type Vector%202D%20Structure) (ElapsedSeconds :type Float%20%28double-precision%29) (TriggeredSeconds :type Float%20%28double-precision%29) (InputAction :type Input%20Action%20Object%20Reference :default "/Game/test/IA_Movetest.IA_Movetest"))
  (Pawn|Input|AddMovementInput (Class|KismetMathLibrary|VectorRight) (.x ActionValue) false)
  (Pawn|Input|AddMovementInput (Class|KismetMathLibrary|VectorForward) (.y ActionValue) false))

(event Input|EnhancedActionEvents|EnhancedInputActionIA_Looktest
  (params (ActionValue :type Vector%202D%20Structure) (ElapsedSeconds :type Float%20%28double-precision%29) (TriggeredSeconds :type Float%20%28double-precision%29) (InputAction :type Input%20Action%20Object%20Reference :default "/Game/test/IA_Looktest.IA_Looktest"))
  (bind _returnvalue (Transformation|GetActorRotation))
  (bind _result (Math|Float|NegateFloat (.x ActionValue))
    (:%20%20
      (Pawn|SetControlRotation (Variables|Default|GetPlayer%20Controller) (Math|Rotator|MakeRotator (.roll _returnvalue) (.pitch _returnvalue) (Class|KismetMathLibrary|DegAtan2 (.y ActionValue) _result))))))

(event Input|EnhancedActionEvents|EnhancedInputActionIA_Shoottest
  (params (ActionValue :type Boolean) (ElapsedSeconds :type Float%20%28double-precision%29) (TriggeredSeconds :type Float%20%28double-precision%29) (InputAction :type Input%20Action%20Object%20Reference :default "/Game/test/IA_Shoottest.IA_Shoottest"))
  (:Started
    (bind _returnvalue (Game|SpawnActorfromClass "/Game/test/BP_testBullet.BP_testBullet_C" (Transformation|GetWorldTransform (Variables|Default|GetScene)) "Undefined" "MultiplyWithRoot" 0 0))
    (Actor|SetOwner _returnvalue self)))

(event Input|EnhancedActionEvents|EnhancedInputActionIA_Jumptest
  (params (ActionValue :type Boolean) (ElapsedSeconds :type Float%20%28double-precision%29) (TriggeredSeconds :type Float%20%28double-precision%29) (InputAction :type Input%20Action%20Object%20Reference :default "/Game/test/IA_Jumptest.IA_Jumptest"))
  (Character|Jump))

(event EventBeginPlay
  (Utilities|FlowControl|DelayUntilNextTick)
  (Variables|Default|SetPlayer%20Controller (Pawn|GetController))
  (Variables|Default|SetGame%20Mode (Game|GetGameMode)))

(event Collision|EventActorBeginOverlap
  (params (OtherActor :type Actor%20Object%20Reference)))

(event EventTick
  (params (DeltaSeconds :type Float%20%28single-precision%29)))

(fn ConstructionScript)